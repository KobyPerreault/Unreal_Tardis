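; BP_Console is a TARDIS console Blueprint that animates its time rotor.
; A Flight event plays one timeline to raise the rotor and reverses a second to lower it, both lerping its relative height.
; The cycle loops through a DoN node up to five times, with no reset wired.
; Tick independently spins the rotor by a fixed step each frame, not scaled by delta time.
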(event `Flight`
  (bind _counter (`/Engine/EditorBlueprintResources/StandardMacros.Do N` 5 :!label _label)
    (:`Exit`
      (bind (_direction _alpha) (`Timeline|RotorUp/Down` :!via `PlayFromStart`)
        (:`Update`
          (`SceneComponent.K2_SetRelativeLocation` (`self.Time_Rotor`) (`KismetMathLibrary.MakeVector` 0.0 0.0 (`KismetMathLibrary.Lerp` 0.0 25.0 _alpha)) false false))
        (:`Finished`
          (bind (_direction_2 _alpha_2) (`Timeline|Timeline` :!via `ReverseFromEnd`)
            (:`Update`
              (`SceneComponent.K2_SetRelativeLocation` (`self.Time_Rotor`) (`KismetMathLibrary.MakeVector` 0.0 0.0 (`KismetMathLibrary.Lerp` 0.0 25.0 _alpha_2)) false false))
            (:`Finished`
              (if (not (>= _counter 5))
                (goto _label)))))))))

(event `self.ReceiveTick`
  (params (DeltaSeconds :type "Float (single-precision)"))
  (`SceneComponent.K2_AddLocalRotation` (`self.Time_Rotor`) (struct :`Yaw` 0.1) false false))

(fn `UserConstructionScript`)