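; BP_Flight_Switch is a TARDIS console lever that triggers flight when interacted with.
; Interact calls PullLever, then finds the first BP_Console in the level through GetAllActorsOfClass and calls its Flight function.
; An unconnected node chain that would call DoorOpenClose on the Tardis actor remains in the graph and never runs.
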(event `/Game/Interact_Interface.Interact`
  (`self.PullLever`)
  (bind _outactors (`GameplayStatics.GetAllActorsOfClass` "/Game/Tardis_Stuff/Console/BPs/BP_Console.BP_Console_C"))
  (bind _asbp_console (cast `/Game/Tardis_Stuff/Console/BPs/BP_Console` (`|GetArrayItem` _outactors)))
  (`/Game/Tardis_Stuff/Console/BPs/BP_Console.Flight` _asbp_console))

(fn `UserConstructionScript`
  (`parent.UserConstructionScript`))