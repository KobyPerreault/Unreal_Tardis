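; BP_Light is a TARDIS console light Blueprint that switches two rect lights on and off through a ToggleLights event.
; The event branches on LightsOn, which flips when the chosen timeline finishes.
; The Fade timeline drives intensity from zero to full when turning on.
; The turn-off branch plays a separate timeline in reverse, but its lerp alpha is fixed at zero, so intensity drops immediately instead of fading.
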(event `Toggle Lights`
  (if (`self.LightsOn`)
    (`Timeline|Timeline` :!via `ReverseFromEnd`
      (:`Update`
        (`LightComponent.SetIntensity` (`self.RectLight1`) (`KismetMathLibrary.Lerp` 0.0 5000.0))
        (`LightComponent.SetIntensity` (`self.RectLight`) (`KismetMathLibrary.Lerp` 0.0 5000.0)))
      (:`Finished`
        (set `self.LightsOn` false)))
    (else
      (bind (_direction _newtrack_0) (`Timeline|Fade` :!via `PlayFromStart`)
        (:`Update`
          (`LightComponent.SetIntensity` (`self.RectLight1`) (`KismetMathLibrary.Lerp` 0.0 5000.0 _newtrack_0))
          (`LightComponent.SetIntensity` (`self.RectLight`) (`KismetMathLibrary.Lerp` 0.0 5000.0 _newtrack_0)))
        (:`Finished`
          (set `self.LightsOn` true))))))

(fn `UserConstructionScript`)